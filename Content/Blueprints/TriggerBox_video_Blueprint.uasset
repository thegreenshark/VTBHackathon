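; A trigger box that sends the VTBOT helper bot to an event point when the first-person character enters it.
; On overlap it finds the bot, hands it the BotBaseActorPoint location and rotation, raises its IsOnEventPoint flag and plays the box's Sound through the bot's audio component.
; On exit it clears the flag, stops that audio and stops the Video, which this graph never starts.
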(event EventBeginPlay)

(event Collision|EventActorBeginOverlap
  (params (OtherActor :type Actor%20Object%20Reference))
  (bind _bot_base_actor_point (Variables|Default|Getbot_base_actor_point))
  (Utilities|Casting|CastToFirstPersonCharacter OtherActor)
  (bind _returnvalue (Actor|GetActorOfClass "/Game/Blueprints/VTBOT_Blueprint.VTBOT_Blueprint_C"))
  (Utilities|FlowControl|Sequence
    (:then_0
      (Variables|/Game/Blueprints/VTBOT_Blueprint.VTBOT_Blueprint_C|SetTargetStopRotation _returnvalue (Transformation|GetActorRotation _bot_base_actor_point)))
    (:then_1
      (Variables|/Game/Blueprints/VTBOT_Blueprint.VTBOT_Blueprint_C|SetTargetStopPoint _returnvalue (Transformation|GetActorLocation _bot_base_actor_point)))
    (:then_2
      (Variables|/Game/Blueprints/VTBOT_Blueprint.VTBOT_Blueprint_C|SetIsOnEventPoint _returnvalue (Variables|Default|Getbool_true)))
    (:then_3
      (Variables|/Script/Engine.AudioComponent|SetSound (Actor|GetComponentbyClass _returnvalue "/Script/Engine.AudioComponent") (Variables|Default|Getsound))
      (Audio|Components|Audio|Play (Actor|GetComponentbyClass _returnvalue "/Script/Engine.AudioComponent") 0.0))))

(event EventTick
  (params (DeltaSeconds :type Float%20%28single-precision%29)))

(event Collision|EventActorEndOverlap
  (params (OtherActor :type Actor%20Object%20Reference))
  (Utilities|Casting|CastToFirstPersonCharacter OtherActor)
  (Default|StopVideo (Variables|Default|Getvideo))
  (bind _returnvalue (Actor|GetActorOfClass "/Game/Blueprints/VTBOT_Blueprint.VTBOT_Blueprint_C"))
  (Variables|/Game/Blueprints/VTBOT_Blueprint.VTBOT_Blueprint_C|SetIsOnEventPoint _returnvalue (Variables|Default|Getbool_false))
  (Audio|Components|Audio|Stop (Actor|GetComponentbyClass (stale Collision|EventActorBeginOverlap _returnvalue) "/Script/Engine.AudioComponent")))

(fn ConstructionScript)