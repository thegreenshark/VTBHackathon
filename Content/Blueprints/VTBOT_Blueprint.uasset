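; VTBOT is a companion robot that follows the player or holds at an event point.
; Each Tick it checks IsOnEventPoint: when set, it interpolates location toward TargetStopPoint and sets rotation by interpolating from TargetStopRotation toward its current rotation.
; Otherwise it uses movement input to chase a raised point offset along the player's angled forward vector, smoothly turning to face back along that vector.
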(event EventBeginPlay)

(event Collision|EventActorBeginOverlap
  (params (OtherActor :type Actor%20Object%20Reference)))

(event EventTick
  (params (DeltaSeconds :type Float%20%28single-precision%29))
  (bind _returnvalue (Utilities|Time|GetWorldDeltaSeconds))
  (bind _returnvalue_2 (Game|GetPlayerCharacter 0))
  (bind _returnvalue_3 (Transformation|GetActorLocation))
  (bind _returnvalue_4 (Utilities|Time|GetWorldDeltaSeconds))
  (bind _returnvalue_5 (Transformation|GetActorRotation _returnvalue_2))
  (bind _returnvalue_6 (Math|Rotator|CombineRotators _returnvalue_5 "0,30.000000, 0"))
  (bind _returnvalue_7 (Math|Vector|GetForwardVector _returnvalue_6))
  (Utilities|FlowControl|Sequence
    (:then_0
      (if (Variables|Default|GetIsOnEventPoint)
        (Transformation|SetActorLocationAndRotation (Math|Interpolation|VInterpTo (Transformation|GetActorLocation) (Variables|Default|GetTargetStopPoint) _returnvalue_4 (* (Variables|Default|GetBotSpeed) 0.3)) (Math|Interpolation|RInterpTo (Variables|Default|GetTargetStopRotation) (Transformation|GetActorRotation) _returnvalue_4 (Variables|Default|GetBotRotationSpeed)))
        (else
          (Pawn|Input|AddMovementInput (- (Math|Interpolation|VInterpTo _returnvalue_3 (+ "0, 0,70.000000" (+ (Transformation|GetActorLocation _returnvalue_2) (* _returnvalue_7 (Variables|Default|GetBotOffsetLen)))) _returnvalue (Variables|Default|GetBotSpeed)) _returnvalue_3) 0.09 false)
          (Transformation|SetActorRotation (Math|Interpolation|RInterpTo (Transformation|GetActorRotation) (Math|Conversions|RotationFromXVector (* _returnvalue_7 -1.0)) _returnvalue (Variables|Default|GetBotRotationSpeed))))))))

(fn ConstructionScript)