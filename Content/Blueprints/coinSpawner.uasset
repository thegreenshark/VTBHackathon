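; Coin spawner actor that drops objects in the level whenever the player character fires its spawn-coin event.
; On BeginPlay it binds to that event on the first-person character, then spawns the configured class just below its own location, always ignoring collision.
; Spawned actors are tracked in an array, and the oldest are destroyed first whenever the count exceeds a configurable maximum.
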(event Custom|spawnCoint
  (bind _spawnedobjectarray (Variables|Default|GetSpawnedObjectArray))
  (bind _returnvalue (Game|SpawnActorfromClass (Variables|Default|GetSpawnedObject) (Math|Conversions|ToTransform(Vector) (+ (Transformation|GetActorLocation) "0, 0,-30.000000")) "AlwaysSpawn" self 0))
  (Utilities|Array|Add (Variables|Default|GetSpawnedObjectArray) _returnvalue)
  (while (> (Utilities|Array|Length (Variables|Default|GetSpawnedObjectArray)) (Variables|Default|GetmaxObjectsCount))
    (Actor|DestroyActor (Utilities|Array|Get(acopy) _spawnedobjectarray))
    (Utilities|Array|RemoveIndex _spawnedobjectarray)))

(event EventBeginPlay
  (bind _asfirst_person_character (Utilities|Casting|CastToFirstPersonCharacter (Game|GetPlayerCharacter 0)))
  (EventDispatchers|BindEventtoSpawnCoin _asfirst_person_character (delegate Custom|spawnCoint)))

(fn ConstructionScript)