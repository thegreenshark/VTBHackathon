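; MoveObject is an actor that moves back and forth between its starting location and the location of a MoveToPosition reference.
; The construction script records the start location, and calling Move while idle starts travel toward whichever end it is not at.
; Each Tick, UpdateMove steps an alpha by a fixed, frame-rate-dependent increment, sets the location with an EaseInOut blend, and returns to idle at either end.
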(event EventBeginPlay)

(event Collision|EventActorBeginOverlap
  (params (OtherActor :type Actor%20Object%20Reference)))

(event EventTick
  (params (DeltaSeconds :type Float%20%28single-precision%29))
  (CallFunction|UpdateMove))

(fn ConstructionScript
  (Variables|Default|SetinitialPos (Transformation|GetActorLocation))
  (Variables|Default|SetmovableStatus "NewEnumerator0"))

(fn Move
  (if (Utilities|Enum|Equal(Enum) (Variables|Default|GetmovableStatus) "NewEnumerator0")
    (if (== (Variables|Default|GeteaseAlpha) 0.0)
      (Variables|Default|SetmovableStatus "NewEnumerator1")
      (else
        (Variables|Default|SetmovableStatus "NewEnumerator2")))))

(fn UpdateMove
  (if (Utilities|Enum|Equal(Enum) (Variables|Default|GetmovableStatus) "NewEnumerator1")
    (bind _output_get (Variables|Default|SeteaseAlpha (+ (Variables|Default|GeteaseAlpha) (Variables|Default|GetincrementStep))))
    (if (>= _output_get 1.0)
      (Variables|Default|SeteaseAlpha 1.0)
      (Variables|Default|SetmovableStatus "NewEnumerator0" :!label _label))
    (Transformation|SetActorLocation (Math|Interpolation|Ease "EaseInOut" (Variables|Default|GeteaseAlpha) (Variables|Default|GetinitialPos) (Transformation|GetWorldLocation (Variables|/Script/Engine.Actor|GetRootComponent (Variables|Default|GetmoveToPosition))) 2.0) false false :!label _label_2)
    (elif (Utilities|Enum|Equal(Enum) (Variables|Default|GetmovableStatus) "NewEnumerator2")
      (bind _output_get_2 (Variables|Default|SeteaseAlpha (- (Variables|Default|GeteaseAlpha) (Variables|Default|GetincrementStep))))
      (if (<= _output_get_2 0.0)
        (Variables|Default|SeteaseAlpha 0.0)
        (goto _label)
        (else
          (goto _label_2))))))